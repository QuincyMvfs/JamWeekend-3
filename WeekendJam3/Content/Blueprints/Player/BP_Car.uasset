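; BP_Car is a car actor that animates its wheels and tilts its body to match the ground.
; While Velocity is non-zero, the async physics tick spins all four wheels and sphere-traces downward.
; The first hit that is not BP_ThirdPersonCharacter feeds GetCarRotationIK, which converts the surface normal into slope angles for BaseCar.
; TurnFrontWheels applies fixed, direction-signed yaw steps to the front wheels and pitch steps to all four.
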(event `self.ReceiveAsyncPhysicsTick`
  (params (DeltaSeconds :type "Float (single-precision)") (SimSeconds :type "Float (single-precision)"))
  (bind _returnvalue (`self.K2_GetActorLocation` self))
  (bind _returnvalue_x (`KismetMathLibrary.BreakVector` (* (`self.DefaultRotationSpeed`) (`self.Velocity`))))
  (if (!= (`self.Velocity`) 0.0)
    (`SceneComponent.K2_AddRelativeRotation` (`self.RearL`) (`KismetMathLibrary.MakeRotator` _returnvalue_x) false false)
    (`SceneComponent.K2_AddRelativeRotation` (`self.FrontL`) (`KismetMathLibrary.MakeRotator` _returnvalue_x) false false)
    (`SceneComponent.K2_AddRelativeRotation` (`self.RearR`) (`KismetMathLibrary.MakeRotator` _returnvalue_x) false false)
    (`SceneComponent.K2_AddRelativeRotation` (`self.FrontR`) (`KismetMathLibrary.MakeRotator` _returnvalue_x) false false)
    (bind (_outhits _returnvalue_2) (`KismetSystemLibrary.SphereTraceMulti` _returnvalue (- _returnvalue (0.0 0.0 100.0)) 1.0 "TraceTypeQuery1"))
    (if _returnvalue_2
      (for _array_element _outhits
        (bind (_bblockinghit _binitialoverlap _time _distance _location _impactpoint _normal _impactnormal _physmat _hitactor) (`GameplayStatics.BreakHitResult` _array_element))
        (if (!= (`GameplayStatics.GetObjectClass` _hitactor) "/Game/Blueprints/Player/BP_ThirdPersonCharacter.BP_ThirdPersonCharacter_C")
          (`SceneComponent.K2_SetWorldRotation` (`self.BaseCar`) (`self.GetCarRotationIK` _normal) false false)
          (break))))))

(event `TurnFrontWheels`
  (params (Direction :type Integer))
  (bind _frontr (`self.FrontR`))
  (bind _frontl (`self.FrontL`))
  (if (> Direction 0)
    (`SceneComponent.K2_AddRelativeRotation` _frontl (struct :`Yaw` 25.0) false false)
    (`SceneComponent.K2_AddRelativeRotation` (`self.FrontR`) (struct :`Yaw` 25.0) false false)
    (`SceneComponent.K2_AddRelativeRotation` _frontr (struct :`Pitch` 20.0) false false)
    (`SceneComponent.K2_AddRelativeRotation` (`self.RearR`) (struct :`Pitch` 20.0) false false)
    (`SceneComponent.K2_AddRelativeRotation` (`self.FrontL`) (struct :`Pitch` 20.0) false false)
    (`SceneComponent.K2_AddRelativeRotation` (`self.RearL`) (struct :`Pitch` 20.0) false false)
    (else
      (`SceneComponent.K2_AddRelativeRotation` _frontl (struct :`Yaw` -25.0) false false)
      (`SceneComponent.K2_AddRelativeRotation` (`self.FrontR`) (struct :`Yaw` -25.0) false false)
      (`SceneComponent.K2_AddRelativeRotation` _frontr (struct :`Pitch` -20.0) false false)
      (`SceneComponent.K2_AddRelativeRotation` (`self.RearR`) (struct :`Pitch` -20.0) false false)
      (`SceneComponent.K2_AddRelativeRotation` (`self.FrontL`) (struct :`Pitch` -20.0) false false)
      (`SceneComponent.K2_AddRelativeRotation` (`self.RearL`) (struct :`Pitch` -20.0) false false))))

(fn `GetCarRotationIK`
  (params (Normal :type "Vector Structure"))
  (returns (NewRotation :type "Rotator Structure"))
  (bind (_returnvalue_roll _returnvalue_pitch _returnvalue_yaw) (`KismetMathLibrary.BreakRotator` (`self.K2_GetActorRotation` self)))
  (bind (_outslopepitchdegreeangle _outsloperolldegreeangle) (`KismetMathLibrary.GetSlopeDegreeAngles` (`self.GetActorRightVector` self) Normal (`self.GetActorUpVector` self)))
  (return (`KismetMathLibrary.MakeRotator` (* _outslopepitchdegreeangle -1.0) (* _outsloperolldegreeangle -1.0) (- _returnvalue_yaw 90.0))))

(fn `UserConstructionScript`)