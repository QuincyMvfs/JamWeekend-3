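; Speed boost pickup that changes the speed of whatever picks it up.
; On pickup, it passes its boost multiplier to the target's UpdateSpeed and spawns an explosion particle effect at the mesh location.
; It then clears its spinning timer and destroys itself.
; The spin logic is not set up in this graph, and the construction script only calls the parent.
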(event `self.OnPickup`
  (params (Target :type "/Game/Blueprints/Player/BP_ThirdPersonCharacter Object Reference"))
  (`/Game/Blueprints/Player/BP_ThirdPersonCharacter.UpdateSpeed` Target (`self.Speed Boost Multiplier`))
  (`GameplayStatics.SpawnEmitterAtLocation` "/Game/StarterContent/Particles/P_Explosion.P_Explosion" (`SceneComponent.K2_GetComponentLocation` (`self.PickupMesh`)))
  (`KismetSystemLibrary.K2_ClearAndInvalidateTimerHandle` (`self.SpinningTimer`))
  (`self.K2_DestroyActor`))

(fn `UserConstructionScript`
  (`parent.UserConstructionScript`))