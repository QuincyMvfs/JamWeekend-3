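; BP_ScorePickup is a spinning pickup that adds score when the third-person character overlaps its collider.
; A looping timer started on BeginPlay rotates the mesh in place of Tick.
; On pickup it updates the score tracker in the character's HUD, spawns an explosion effect, clears the timer and destroys itself.
; It caches the game instance but never uses it, though the spin only starts if that cast succeeds.
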(event `self.ReceiveBeginPlay`
  ;[0 0 0] Game Instance
  (bind _asbp_default_game_instance (cast `/Game/Blueprints/Core/BP_Default_GameInstance` (`GameplayStatics.GetGameInstance`)))
  (set `self.GameInstanceRef` _asbp_default_game_instance)
  ;[0 0 0] Spinning Loop
  (bind _returnvalue (`KismetSystemLibrary.K2_SetTimerDelegate` (delegate `SpinningLoop`) 0.025 true))
  (set `self.SpinningTimer` _returnvalue))

(event `SpinningLoop`
  ;[0 0 0] Spinning Loop
  (`SceneComponent.K2_AddRelativeRotation` (`self.PickupMesh`) (struct :`Yaw` 5.0) false false))

(event `self.PickupCollider.OnComponentBeginOverlap`
  (params (OverlappedComponent :type "PrimitiveComponent Object Reference") (OtherActor :type "Actor Object Reference") (OtherComp :type "PrimitiveComponent Object Reference") (OtherBodyIndex :type Integer) (bFromSweep :type Boolean) (SweepResult :type "HitResult Structure (by ref)"))
  (bind _asbp_third_person_character (cast `/Game/Blueprints/Player/BP_ThirdPersonCharacter` OtherActor))
  (`self.OnPickup` _asbp_third_person_character))

(event `OnPickup`
  (params (Target :type "/Game/Blueprints/Player/BP_ThirdPersonCharacter Object Reference"))
  (`/Game/Blueprints/UI/Panels/WBP_ScoreTracker.UpdateScore` (`/Game/Blueprints/UI/Menus/WBP_GameplayHud.WBP_ScoreTracker` (`/Game/Blueprints/Player/BP_ThirdPersonCharacter.GameplayHud` Target)) (`self.ScoreToAdd`))
  (`GameplayStatics.SpawnEmitterAtLocation` "/Game/StarterContent/Particles/P_Explosion.P_Explosion" (`SceneComponent.K2_GetComponentLocation` (`self.PickupMesh`)))
  (`KismetSystemLibrary.K2_ClearAndInvalidateTimerHandle` (`self.SpinningTimer`))
  (`self.K2_DestroyActor`))

(fn `UserConstructionScript`)