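; Level-end trigger volume that finishes the level when the third-person character overlaps its box.
; On overlap it stops the HUD speedrun timer, calls LevelCompleted and hides the gameplay HUD.
; It then shows the victory screen widget with UI-only input and a visible cursor, and disables gravity and physics simulation on the character's capsule.
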(event `self.Box.OnComponentBeginOverlap`
  (params (OverlappedComponent :type "PrimitiveComponent Object Reference") (OtherActor :type "Actor Object Reference") (OtherComp :type "PrimitiveComponent Object Reference") (OtherBodyIndex :type Integer) (bFromSweep :type Boolean) (SweepResult :type "HitResult Structure (by ref)"))
  (bind _returnvalue (`GameplayStatics.GetPlayerController` 0))
  (bind _asbp_third_person_character (cast `/Game/Blueprints/Player/BP_ThirdPersonCharacter` OtherActor))
  (`/Game/Blueprints/UI/Panels/WBP_SpeedrunTimer.StopTimer` (`/Game/Blueprints/UI/Menus/WBP_GameplayHud.WBP_SpeedrunTimer` (`/Game/Blueprints/Player/BP_ThirdPersonCharacter.GameplayHud` _asbp_third_person_character)))
  (`self.LevelCompleted`)
  (`/Game/Blueprints/UI/Menus/WBP_GameplayHud.HideAll` (`/Game/Blueprints/Player/BP_ThirdPersonCharacter.GameplayHud` _asbp_third_person_character))
  (bind _returnvalue_2 (`|CreateWidget` "/Game/Blueprints/UI/Menus/WBP_VictoryScreen.WBP_VictoryScreen_C" _returnvalue))
  (`UserWidget.AddToViewport` _returnvalue_2 0)
  (`WidgetBlueprintLibrary.SetInputMode_UIOnlyEx` _returnvalue _returnvalue_2)
  (set `PlayerController.bShowMouseCursor` true _returnvalue)
  (bind _capsulecomponent (`Character.CapsuleComponent` _asbp_third_person_character))
  (`PrimitiveComponent.SetEnableGravity` _capsulecomponent false)
  (`PrimitiveComponent.SetSimulatePhysics` _capsulecomponent false))

(fn `UserConstructionScript`)